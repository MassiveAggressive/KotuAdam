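; Lobby game mode that tracks connected players and launches the match as a listen server.
; BeginPlay creates the lobby widget with the first player's banner and switches to UI-only input; later joiners are added to the player list and get banners.
; Logout drops players from the list without updating banners.
; StartGame requires a minimum player count, opens DevMap, then calls MapChangedMessage on each player.
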(event EventOnLogout
  (params (ExitingController :type Controller%20Object%20Reference))
  (Development|PrintString (Utilities|GetDisplayName ExitingController))
  (Utilities|Array|RemoveItem (Variables|Default|GetPlayers) (.AsPlayer%20Controller (Utilities|Casting|CastToPlayerController ExitingController))))

(event EventStartGame
  (if (>= (Utilities|Array|Length (Variables|Default|GetPlayers)) (Variables|Default|GetNeededPlayerAmount))
    (Game|OpenLevel(byObjectReference) "/Game/Maps/DevMap.DevMap" true "listen")
    (for _array_element (Variables|Default|GetPlayers)
      (Class|BPIPlayerController|MapChanged(Message) _array_element))))

(event EventBeginPlay
  (bind _returnvalue (UserInterface|CreateWidget "/Game/Blueprints/GameMode/Widget/W_Lobby.W_Lobby_C"))
  (bind _output_get (Variables|Default|SetW_Lobby _returnvalue))
  (UserInterface|Viewport|AddtoViewport _output_get 0)
  (Default|AddPlayerBanner _output_get (Class|AdvancedSessionsLibrary|GetPlayerName (Utilities|Array|Get(acopy) (Variables|Default|GetPlayers))))
  (Input|SetInputModeUIOnly (Game|GetPlayerController 0) (Variables|Default|GetW_Lobby) "DoNotLock"))

(event EventHandleStartingNewPlayer
  (params (NewPlayer :type Player%20Controller%20Object%20Reference))
  (Utilities|Array|Add (Variables|Default|GetPlayers) NewPlayer)
  (bind _w_lobby (Variables|Default|GetW_Lobby)
    (:then
      (Default|AddPlayerBanner _w_lobby (Class|AdvancedSessionsLibrary|GetPlayerName NewPlayer)))
    (:else)))

(fn ConstructionScript
  (|CallParentFunction))