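; Multiplayer game instance that manages online session hosting, search, joining and teardown, along with the main menu widget.
; Creating a session tags it with a game name and opens the lobby as a listen server.
; Search results go back to the requesting widget, and joining hides the menu and stores the session.
; Destroying a session returns to the main menu map, and shutdown also destroys it.
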(event EventCreateSession
  (params (GameName :type String))
  (|AdvancedSession (Utilities|Array|MakeArray (Class|AdvancedSessionsLibrary|MakeLiteralSessionPropertyString "GameName" GameName)) (Game|GetPlayerController 0) 8 8 false true false true true true false true false true
    (:then
      (Development|PrintString "Create Execute"))
    (:OnSuccess
      (Development|PrintString "Create Success")
      (Game|OpenLevel(byObjectReference) "/Game/Maps/M_Lobby.M_Lobby" true "listen")
      (CallFunction|HideMainMenu))
    (:OnFailure
      (Development|PrintString "Create Failure"))))

(event EventShowMainMenu
  (Variables|Default|GetW_MainMenu
    (:then
      _)
    (:else
      (bind _returnvalue (UserInterface|CreateWidget "/Game/Blueprints/GameMode/Widget/W_MainMenu.W_MainMenu_C"))
      (bind _output_get (Variables|Default|SetW_MainMenu _returnvalue))))
  (UserInterface|Viewport|AddtoViewport _output_get 0)
  (Input|SetInputModeUIOnly (Game|GetPlayerController 0) (Variables|Default|GetW_MainMenu) "DoNotLock"))

(event EventHideMainMenu
  (bind _w_mainmenu (Variables|Default|GetW_MainMenu)
    (:then
      (Widget|RemovefromParent _w_mainmenu))
    (:else)))

(event EventDestroySession
  (|DestroySession (Game|GetPlayerController 0)
    (:then
      (Development|PrintString "Destroy Session Execute"))
    (:OnSuccess
      (Development|PrintString "Destroy Session Successful")
      (Game|OpenLevel(byObjectReference) "/Game/Maps/M_MainMenu.M_MainMenu")
      (CallFunction|ShowMainMenu))
    (:OnFailure
      (Development|PrintString "Destroy Session Failure"))))

(event EventFindSession
  (params (AffectedWidget :type W%20Find%20Session%20Object%20Reference))
  (bind _results (|FindSessionsAdvanced (Game|GetPlayerController 0) 100 false "ClientServersOnly" 0 false false false true)
    (:then
      (Development|PrintString "Find Execute"))
    (:OnSuccess
      (Development|PrintString "Find Success")
      (Default|SessionFound AffectedWidget _results))
    (:OnFailure
      (Development|PrintString "Find Failure"))))

(event EventJoinSession
  (params (Session :type Blueprint%20Session%20Result%20Structure))
  (|JoinSession (Game|GetPlayerController 0) Session
    (:then
      (CallFunction|HideMainMenu)
      (CallFunction|SetCurrentSession Session))))

(event EventShutdown
  (|DestroySession (Game|GetPlayerController 0)))

(fn GetCurrentSession
  (return (Variables|Default|GetCurrentSession)))

(fn GetMainMenuWidget
  (return (Variables|Default|GetW_MainMenu)))